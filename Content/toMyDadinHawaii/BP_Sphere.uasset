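; BP_Sphere is a sphere actor that explodes and awards points when it is destroyed.
; A Params struct drives its scale, its color and its score value.
; BeginPlay applies the scale and sets the Color parameter on a dynamic material instance of the mesh.
; Destroyed spawns the P_Explosion emitter at its location and passes the score to the BP_Score actor found with GetActorOfClass.
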(event `self.ReceiveBeginPlay`
  (bind _sphere (`self.Sphere`))
  (bind (_score _color _scale) (break `/Game/VRTemplate/Blueprints/BPS_Sphere` (`self.Params`)))
  (`self.SetActorScale3D` _scale)
  (bind _returnvalue (`PrimitiveComponent.CreateDynamicMaterialInstance` _sphere 0 (`PrimitiveComponent.GetMaterial` _sphere 0) "None"))
  (`MaterialInstanceDynamic.SetVectorParameterValue` _returnvalue "Color" _color))

(event `self.ReceiveDestroyed`
  (`GameplayStatics.SpawnEmitterAtLocation` "/Game/StarterContent/Particles/P_Explosion.P_Explosion" (`self.K2_GetActorLocation`))
  (bind _returnvalue (`GameplayStatics.GetActorOfClass` "/Game/toMyDadinHawaii/BP_Score.BP_Score_C"))
  (`/Game/toMyDadinHawaii/BP_Score.OnAddScore` _returnvalue (`.Score_2_37E8055741B2426CFA353F9A42FFB529` (break `/Game/VRTemplate/Blueprints/BPS_Sphere` (`self.Params`)))))

(fn `UserConstructionScript`)