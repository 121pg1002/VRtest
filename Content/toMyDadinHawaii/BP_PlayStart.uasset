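; BP_PlayStart is a short-lived actor that kicks off gameplay two seconds after it begins play.
; It destroys itself after that delay and uses its Destroyed event as the start trigger.
; That event starts the BP_SphereSpawnManager spawn timer, calls OnStart on the W_Time widget held by BP_Time, and plays the background music.
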(event `self.ReceiveBeginPlay`
  (`KismetSystemLibrary.Delay` 2.0)
  (`self.K2_DestroyActor`))

(event `self.ReceiveDestroyed`
  (bind _returnvalue (`GameplayStatics.GetActorOfClass` "/Game/toMyDadinHawaii/BP_SphereSpawnManager.BP_SphereSpawnManager_C"))
  (`/Game/toMyDadinHawaii/BP_SphereSpawnManager.OnStartSpawnTimer` _returnvalue)
  (bind _returnvalue_2 (`GameplayStatics.GetActorOfClass` "/Game/toMyDadinHawaii/BP_Time.BP_Time_C"))
  (bind _asw_time (cast `/Game/toMyDadinHawaii/W_Time` (`WidgetComponent.GetWidget` (`/Game/toMyDadinHawaii/BP_Time.Widget` _returnvalue_2))))
  (`/Game/toMyDadinHawaii/W_Time.OnStart` _asw_time)
  (`GameplayStatics.PlaySound2D` "/Game/toMyDadinHawaii/Sound/BGM_Cue.BGM_Cue" 1.0 1.0 0.0 null null))

(fn `UserConstructionScript`)