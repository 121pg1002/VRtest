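; BP_SphereSpawnManager spawns scoring BP_Sphere actors at random positions while spawning is active.
; OnStartSpawnTimer starts a looping timer that calls OnSpawnSphere, and OnEndSpawn clears it through the stored handle.
; Each spawn passes one of four randomly chosen sphere parameter structs, pairing higher scores with smaller scales and distinct colors.
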(event `self.ReceiveBeginPlay`)

(event `OnStartSpawnTimer`
  (bind _returnvalue (`KismetSystemLibrary.K2_SetTimerDelegate` (delegate `OnSpawnSphere`) 0.7 true))
  (set `self.TimerHandle` _returnvalue))

(event `OnSpawnSphere`
  ;[1 1 1] スフィアを生成
  (`|SpawnActorFromClass` "/Game/toMyDadinHawaii/BP_Sphere.BP_Sphere_C" (`KismetMathLibrary.MakeTransform` (`KismetMathLibrary.MakeVector` (`KismetMathLibrary.RandomFloatInRange` 900.0 500.0) (`KismetMathLibrary.RandomFloatInRange` -500.0 500.0) (`KismetMathLibrary.RandomFloatInRange` 100.0 300.0))) "Undefined" "OverrideRootScale" null (select `int` (`KismetMathLibrary.RandomIntegerInRange` 0 3) :`0` (make `/Game/VRTemplate/Blueprints/BPS_Sphere` 10.0 (struct :`R` 1.0 :`G` 1.0 :`B` 1.0 :`A` 1.0)) :`1` (make `/Game/VRTemplate/Blueprints/BPS_Sphere` 30.0 (struct :`R` 1.0 :`G` 0.458214 :`A` 1.0) (0.7 0.7 0.7)) :`2` (make `/Game/VRTemplate/Blueprints/BPS_Sphere` 50.0 (struct :`R` 1.0 :`B` 0.93668 :`A` 1.0) (0.3 0.3 0.3)) :`3` (make `/Game/VRTemplate/Blueprints/BPS_Sphere` 100.0 (struct :`R` 1.0 :`G` 0.017051 :`A` 1.0) (0.1 0.1 0.1))) null))

(event `OnEndSpawn`
  (`KismetSystemLibrary.K2_ClearAndInvalidateTimerHandle` (`self.TimerHandle`)))

(fn `UserConstructionScript`)