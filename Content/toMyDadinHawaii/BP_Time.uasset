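; BP_Time is a Blueprint that hosts a time display widget, W_Time, and controls the visibility of its text.
; SetVisibility casts the Widget component's widget to W_Time and passes the requested visibility to its text block.
; The OnAddScore event is empty, and an unconnected fragment that would add to W_Score's score when time drops below zero never runs.
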(event `OnAddScore`
  (params (Value :type "Float (double-precision)")))

(fn `SetVisibility`
  (params (InVisibility :type "ESlateVisibility Enum" :default "Visible"))
  (bind _asw_time (cast `/Game/toMyDadinHawaii/W_Time` (`WidgetComponent.GetWidget` (`self.Widget`))))
  (`Widget.SetVisibility` (`/Game/toMyDadinHawaii/W_Time.TextBlock_0` _asw_time) InVisibility))

(fn `UserConstructionScript`)